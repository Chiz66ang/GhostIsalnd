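; BP_PlaceInLine is a placement actor that lays out copies of one static mesh in a grid of evenly spaced rows.
; The Construction Script uses nested loops to add a StaticMeshComponent per cell, with configurable mesh, rotation, counts and spacing.
; A running relative location steps along X within each row, then resets X and moves along Y for the next, with spacing in 50-unit multiples.
; The event graph is empty.
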(event EventBeginPlay)

(event Collision|EventActorBeginOverlap
  (params (OtherActor :type Actor%20Object%20Reference)))

(event EventTick
  (params (DeltaSeconds :type Float%20%28single-precision%29)))

(fn ConstructionScript
  (for _index (range 0 (- (Variables|Default|GetCountY) 1))
    (for _index_2 (range 0 (- (Variables|Default|GetCount) 1))
      (bind _returnvalue (AddComponent|AddStaticMeshComponent false (Math|Transform|MakeTransform (Variables|Default|GetNewMeshLocation) (Variables|Default|GetRotator))))
      (Components|StaticMesh|SetStaticMesh _returnvalue (Variables|Default|GetStatic%20Mesh))
      (Variables|Default|SetNewMeshLocation (+ (Variables|Default|GetNewMeshLocation) (Math|Vector|MakeVector (* (Variables|Default|GetDistance) 5e+01) 0.0 0.0))))
    (Variables|Default|SetNewMeshLocation (Math|Vector|MakeVector 0.0 (* (+ _index 1) (* (Variables|Default|GetDistanceY) 5e+01)) 0.0))))