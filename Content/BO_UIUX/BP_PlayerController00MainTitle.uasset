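; Player controller for the main title screen that owns the main menu and options widgets.
; BeginPlay creates both widgets, shows the mouse cursor and hides options.
; SetOption toggles visibility between the two.
; A SkillSelect hold slows global time and shows a skill selector, but that widget's creation code is disconnected, as is an input-mapping node.
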(event Custom|SetOption
  (params (Active :type Boolean))
  (bind _optionwidget (Variables|Default|GetOptionWidget))
  (bind _globalpanel (Variables|Default|GetGlobalPanel))
  (if Active
    (Widget|SetVisibility _optionwidget "Visible")
    (Widget|SetVisibility _globalpanel "Hidden")
    (else
      (Widget|SetVisibility _optionwidget "Hidden")
      (Widget|SetVisibility _globalpanel "Visible"))))

(event EventBeginPlay
  (bind _returnvalue (UserInterface|CreateWidget "/Game/BO_UIUX/Widget_01_0Main.Widget_01_0Main_C"))
  (bind _output_get (Variables|Default|SetGlobalPanel _returnvalue))
  (UserInterface|Viewport|AddtoViewport _output_get 0)
  (Variables|/Script/Engine.PlayerController|SetbShowMouseCursor (Game|GetPlayerController 0) true)
  (bind _returnvalue_2 (UserInterface|CreateWidget "/Game/BO_UIUX/Widget_01_2Option.Widget_01_2Option_C"))
  (bind _output_get_2 (Variables|Default|SetOptionWidget _returnvalue_2))
  (UserInterface|Viewport|AddtoViewport _output_get_2 0)
  (Widget|SetVisibility _output_get_2 "Hidden"))

(event Input|ActionEvents|InputActionSkillSelect
  (params (Key :type Key%20Structure))
  (bind _wskillselector (Variables|Default|GetWSkillSelector))
  (:Pressed
    (Widget|SetVisibility _wskillselector "Visible")
    (Utilities|Time|SetGlobalTimeDilation 0.05))
  (:Released
    (Widget|SetVisibility _wskillselector "Hidden")
    (Utilities|Time|SetGlobalTimeDilation 1.0)))

(fn ConstructionScript)