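; Game mode for Level 2 that runs the enemy-clear, boss fight and exit portal flow.
; At start it counts AIMob_Base enemies and caches the tagged boss spawn point and the BossRoomCollision door.
; Each enemy death decrements the count, opening the boss room at zero.
; Separate events spawn Spider_Boss above the spawn point, then remove it, and spawn a TeleportPortal leading to StageS.
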(event Custom|OnEnemyDead
  (bind _result (Math|Integer|DecrementInt (Variables|Default|GetEnemyNum))
    (:%20%20
      (if (<= _result 0)
        (Utilities|FlowControl|Delay 0.2)
        (Default|OpenBossRoom (Variables|Default|GetBossRoomDoor))
        (else
          (Variables|Default|SetEnemyNum _result))))))

(event Custom|ActivatePortal
  (params (SpawnLocation :type Vector))
  (bind _returnvalue (Game|SpawnActorfromClass "/Game/1LEVEL/TeleportPortal.TeleportPortal_C" (Math|Transform|MakeTransform SpawnLocation "0, 0, 0" "1,1,1") "Undefined" 0 0))
  (Variables|/Game/1LEVEL/TeleportPortal.TeleportPortal_C|SetLevelName _returnvalue "StageS"))

(event Custom|CloseDoor%20SpawnBoss
  (bind _bossspawnpoint (Variables|Default|GetBossSpawnPoint))
  (bind _returnvalue (Transformation|GetActorLocation _bossspawnpoint))
  (bind (_x _y _z) (Math|Vector|BreakVector _returnvalue))
  (bind _returnvalue_2 (AI|SpawnAIFromClass "/Game/JS_Character/BossSpider/Spider_Boss.Spider_Boss_C" 0 (Math|Vector|MakeVector _x _y (+ _z 1.5e+02)) (Transformation|GetActorRotation _bossspawnpoint) false))
  (Utilities|FlowControl|Delay 1.0)
  (Utilities|IsValid _returnvalue_2
    (:Is%20Valid
      (Actor|DestroyActor (Variables|Default|GetBossSpawnPoint)))))

(event EventBeginPlay
  (bind _outactors (Actor|GetAllActorsOfClass "/Game/JS_Character/NormalMob/AIMob_Base.AIMob_Base_C"))
  (Variables|Default|SetEnemyNum (Utilities|Array|Length _outactors))
  (bind _outactors_2 (Actor|GetAllActorswithTag "BossSpawnPoint"))
  (Variables|Default|SetBossSpawnPoint (.AsTarget%20Point (Utilities|Casting|CastToTargetPoint (Utilities|Array|Get(acopy) _outactors_2))))
  (bind _outactors_3 (Actor|GetAllActorsOfClass "/Game/1LEVEL/BossRoomCollision.BossRoomCollision_C"))
  (Variables|Default|SetBossRoomDoor (Utilities|Array|Get(acopy) _outactors_3)))

(event EventTick
  (params (DeltaSeconds :type Float%20%28single-precision%29)))

(fn ConstructionScript)